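; Proximity highlight actor that lights up when the player's DefaultPawn_BP comes near and shows a hint on screen.
; A Sphere overlap toggles a SpotLight, which the construction script hides initially.
; Begin and end overlap share one path that passes a pick or search prompt to HUD_BP's DrawTextToScreen.
; Only begin overlap filters for the pawn; any actor leaving turns the light off and changes the prompt.
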(event `self.Sphere.OnComponentBeginOverlap`
  (params (OverlappedComponent :type "PrimitiveComponent Object Reference") (OtherActor :type "Actor Object Reference") (OtherComp :type "PrimitiveComponent Object Reference") (OtherBodyIndex :type Integer) (bFromSweep :type Boolean) (SweepResult :type "HitResult Structure (by ref)"))
  (cast `/Game/BluePrints/DefaultPawn_BP` OtherActor)
  (`SceneComponent.SetVisibility` (`self.SpotLight`) true false)
  (set `self.TEXT` "Pick the highlighted Object")
  (bind _ashud_bp (cast `/Game/BluePrints/HUD_BP` (`PlayerController.GetHUD` (`GameplayStatics.GetPlayerController` 0)) :!label _label))
  (`/Game/BluePrints/HUD_BP.DrawTextToScreen` _ashud_bp true (`self.TEXT`)))

(event `self.Sphere.OnComponentEndOverlap`
  (params (OverlappedComponent :type "PrimitiveComponent Object Reference") (OtherActor :type "Actor Object Reference") (OtherComp :type "PrimitiveComponent Object Reference") (OtherBodyIndex :type Integer))
  (`SceneComponent.SetVisibility` (`self.SpotLight`) false false)
  (set `self.TEXT` "Any object looking special?")
  (goto _label))

(fn `UserConstructionScript`
  (`SceneComponent.SetVisibility` (`self.SpotLight`) false false))