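; HUD Blueprint that shows the game's HUD widget and draws a text prompt on screen.
; BeginPlay creates HUDWidgetBlueprint and adds it to the viewport.
; DrawHUD draws the text in the upper right, positioned relative to viewport size, through a gate that DrawTextToScreen opens or closes.
; The construction script calls DrawTextToScreen with the prompt "Where is that object?".
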(event `self.ReceiveBeginPlay`
  (bind _returnvalue (`|CreateWidget` "/Game/BluePrints/HUDWidgetBlueprint.HUDWidgetBlueprint_C"))
  (`UserWidget.AddToViewport` _returnvalue 0))

(event `self.ReceiveDrawHUD`
  (params (SizeX :type Integer) (SizeY :type Integer))
  (bind (_x _y) (`KismetMathLibrary.BreakVector2D` (`WidgetLayoutLibrary.GetViewportSize`)))
  (`/Engine/EditorBlueprintResources/StandardMacros.Gate` false :!label _label
    (:`Exit`
      (`self.DrawText` (stale `DrawTextToScreen` TEXT) (struct :`R` 1.0 :`G` 1.0 :`B` 1.0 :`A` 1.0) (* _x 0.7) (* _y 0.075) "/Game/Fonts/No_Virus_Font.No_Virus_Font" 2.0))))

(event `DrawTextToScreen`
  (params (bDraw :type Boolean) (TEXT :type String))
  (if bDraw
    (goto _label :!via `Open`)
    (else
      (goto _label :!via `Close`))))

(fn `UserConstructionScript`
  (`self.DrawTextToScreen` true "Where is that object?"))